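; Tank pawn Blueprint that handles the player's in-game HUD and pause menu.
; The G key toggles a game HUD widget, creating a new one each time it is shown and removing it when hidden.
; While the HUD is visible, Tick pushes the tank's suspension distance and strength to it.
; The pause input action adds a new pause menu widget to the viewport without pausing the game here.
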(event Input|EnhancedActionEvents|EnhancedInputActionIA_PauseGame
  (params (ActionValue :type Boolean) (ElapsedSeconds :type Float%20%28double-precision%29) (TriggeredSeconds :type Float%20%28double-precision%29) (InputAction :type Input%20Action%20Object%20Reference :default "/Game/Assets/Input/Actions/IA_PauseGame.IA_PauseGame"))
  (bind _returnvalue (UserInterface|CreateWidget "/Game/Blueprints/Widgets/WBP_PauseMenu.WBP_PauseMenu_C" (Game|GetPlayerController 0)))
  (UserInterface|Viewport|AddtoViewport _returnvalue 0))

(event EventBeginPlay)

(event Collision|EventActorBeginOverlap
  (params (OtherActor :type Actor%20Object%20Reference)))

(event EventTick
  (params (DeltaSeconds :type Float%20%28single-precision%29))
  (bind _hud (Variables|Default|GetHUD))
  (if (and (Variables|Default|GetHUD_Visible) (Utilities|IsValid (Variables|Default|GetHUD)))
    (Default|UpdateSuspensionDistance _hud (Variables|Default|GetSuspensionDistance))
    (Default|UpdateSuspensionStrength _hud (Variables|Default|GetSuspensionStrength))))

(event Input|KeyboardEvents|G
  (params (Key :type Key%20Structure :default "None"))
  (:Pressed
    (if (Variables|Default|GetHUD_Visible)
      (Widget|RemovefromParent (Variables|Default|GetHUD))
      (Variables|Default|SetHUD_Visible false)
      (else
        (bind _returnvalue (UserInterface|CreateWidget "/Game/Blueprints/Widgets/WBP_HUD_Game.WBP_HUD_Game_C" (Game|GetPlayerController 0)))
        (bind _output_get (Variables|Default|SetHUD _returnvalue))
        (UserInterface|Viewport|AddtoViewport _output_get 0)
        (Variables|Default|SetHUD_Visible true)))))

(fn ConstructionScript)